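; BP_CharmHit is a boss skill hit volume that flags charm actors it reaches.
; Every Tick grows the Sphere's world scale by a fixed step, independent of delta time, forming an expanding area.
; When the Sphere begins overlapping a CharmParent, it sets that actor's IsCharmOverlapping flag, then destroys itself after a short delay.
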(event `self.ReceiveBeginPlay`)

(event `self.ReceiveActorBeginOverlap`
  (params (OtherActor :type "Actor Object Reference")))

(event `self.ReceiveTick`
  (params (DeltaSeconds :type "Float (single-precision)"))
  (bind (_returnvalue_x _returnvalue_y _returnvalue_z) (`KismetMathLibrary.BreakVector` (`SceneComponent.K2_GetComponentScale` (`self.Sphere`))))
  (`SceneComponent.SetWorldScale3D` (`self.Sphere`) (`KismetMathLibrary.MakeVector` (+ _returnvalue_x 0.03) (+ _returnvalue_y 0.03) (+ _returnvalue_z 0.03))))

(event `self.Sphere.OnComponentBeginOverlap`
  (params (OverlappedComponent :type "PrimitiveComponent Object Reference") (OtherActor :type "Actor Object Reference") (OtherComp :type "PrimitiveComponent Object Reference") (OtherBodyIndex :type Integer) (bFromSweep :type Boolean) (SweepResult :type "HitResult Structure (by ref)"))
  (bind _ascharm_parent (cast `/Game/Player/Charm/CharmParent` OtherActor))
  (set `/Game/Player/Charm/CharmParent.IsCharmOverlapping` true _ascharm_parent)
  (`KismetSystemLibrary.Delay` 3.0)
  (`self.K2_DestroyActor`))

(fn `UserConstructionScript`)